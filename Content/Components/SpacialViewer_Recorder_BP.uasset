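; Actor component that records its owner's transform over time by leaving Spacial_Viewer_BP actors as visual snapshots.
; Configure stores the settings, and StartRecording starts a looping timer, presumably driving Snapshot, which spawns a viewer at the owner's transform with the chosen display options.
; Snapshot pauses the timer when world delta seconds (not elapsed time) minus Start reaches Duration.
; EndPlay destroys all spawned snapshots.
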(event `Start Recording`
  (bind _returnvalue (`KismetSystemLibrary.K2_SetTimerDelegate` (`|CreateDelegate` :!event `Snapshot`) (`self.Interval`) true))
  (set `self.Timer Handle` _returnvalue))

(event `Snapshot`
  (bind _returnvalue (`self.GetOwner`))
  (if (>= (- (`GameplayStatics.GetWorldDeltaSeconds`) (`self.Start`)) (`self.Duration`))
    (`KismetSystemLibrary.K2_PauseTimerHandle` (`self.Timer Handle`))
    (else
      (bind _returnvalue_2 (`|SpawnActorFromClass` "/Game/Actors/Spacial_Viewer_BP.Spacial_Viewer_BP_C" (`Actor.GetTransform` _returnvalue) "AlwaysSpawn" "OverrideRootScale" _returnvalue null))
      (`KismetArrayLibrary.Array_Add` (`self.Snapshots`) _returnvalue_2)
      (`/Game/Actors/Spacial_Viewer_BP.Show View` _returnvalue_2 (`self.View Option`) (`self.Direction View Mode`) (`self.With Scale`)))))

(event `self.ReceiveEndPlay`
  (params (EndPlayReason :type "EEndPlayReason Enum" :default "Destroyed"))
  (if (> (`KismetArrayLibrary.Array_Length` (`self.Snapshots`)) 0)
    (for _array_element (`self.Snapshots`)
      (`Actor.K2_DestroyActor` _array_element))))

(fn `Configure`
  (params (Interval :type "Float (double-precision)") (Duration :type "Float (double-precision)") (Start :type "Float (double-precision)") (`View Option` :type "/Game/Components/Assets/ESViewer_ViewOption Enum" :default "NewEnumerator3") (`Direction View Mode` :type "/Game/Components/Assets/EDirectionView_Mode Enum" :default "NewEnumerator0") (`With Scale` :type Boolean))
  (`|ExecutionSequence`
    (:`then_0`
      (set `self.Interval` Interval))
    (:`then_1`
      (set `self.Duration` Duration))
    (:`then_2`
      (set `self.Start` Start))
    (:`then_3`
      (set `self.View Option` `View Option`))
    (:`then_4`
      (set `self.Direction View Mode` `Direction View Mode`))
    (:`then_5`
      (set `self.With Scale` `With Scale`))))