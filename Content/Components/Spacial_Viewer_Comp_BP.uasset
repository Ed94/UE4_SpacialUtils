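; Actor component that visualizes the owner's or given position, axes, orientation, scale and transform by spawning SpacialViewer_BP actors.
; BeginPlay spawns a parent viewer attached to the owner, which the plain Show functions use.
; Location, direction and transform variants spawn separate, unattached viewers, all tracked in Viewers and destroyed on EndPlay.
; RecordViews adds a SpacialViewer_Recorder_BP component to the owner, configures its interval, duration and view options, then starts recording.
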(event `self.ReceiveBeginPlay`
  (bind _returnvalue (`self.Make Viewer`))
  (bind _output_get (set `self.Parent_View` _returnvalue))
  (`Actor.K2_AttachToActor` _output_get (`self.GetOwner`) "None" "SnapToTarget" "SnapToTarget" "SnapToTarget" true))

(event `self.ReceiveEndPlay`
  (params (EndPlayReason :type "EEndPlayReason Enum" :default "Destroyed"))
  (for _array_element (`self.Viewers`)
    (`Actor.K2_DestroyActor` _array_element)))

(event `Record Views`
  (params (Interval :type "Float (double-precision)") (Duration :type "Float (double-precision)") (`View Option` :type "EViewMode Enum" :default "Position") (`Direction View Mode` :type "EDirectionViewMode Enum" :default "Vector") (`Use Gnomon` :type Boolean) (`Transform: With Scale` :type Boolean))
  (bind _returnvalue (`|AddComponentByClass` (`self.GetOwner`) "/Game/Components/SpacialViewer_Recorder_BP.SpacialViewer_Recorder_BP_C"))
  (`/Game/Components/SpacialViewer_Recorder_BP.Configure` _returnvalue Interval Duration 0.0 `View Option` `Direction View Mode` `Use Gnomon` `Transform: With Scale`)
  (`/Game/Components/SpacialViewer_Recorder_BP.Start Recording` _returnvalue))

(fn `Make Viewer`
  (returns (ReturnValue :type "/Game/Actors/SpacialViewer_BP Object Reference"))
  (bind _returnvalue (`self.GetOwner`))
  (bind _returnvalue_2 (`|SpawnActorFromClass` "/Game/Actors/SpacialViewer_BP.SpacialViewer_BP_C" (`Actor.GetTransform` _returnvalue) "Undefined" "OverrideRootScale" _returnvalue null))
  (`KismetArrayLibrary.Array_Add` (`self.Viewers`) _returnvalue_2)
  (return _returnvalue_2))

(fn `Make Viewer (With Transform)`
  (params (Transform :type "Transform Structure"))
  (returns (ReturnValue :type "/Game/Actors/SpacialViewer_BP Object Reference"))
  (bind _returnvalue (`|SpawnActorFromClass` "/Game/Actors/SpacialViewer_BP.SpacialViewer_BP_C" Transform "Undefined" "OverrideRootScale" (`self.GetOwner`) null))
  (`KismetArrayLibrary.Array_Add` (`self.Viewers`) _returnvalue)
  (return _returnvalue))

(fn `Show Forward`
  (params (Mode :type "EDirectionViewMode Enum" :default "Vector"))
  (`SpacialViewer.ShowForward` (`self.Parent_View`) Mode))

(fn `Show Forward (At Direction)`
  (params (Direction :type "Rotator Structure (by ref)") (`View Mode` :type "EDirectionViewMode Enum" :default "Vector"))
  (bind _returnvalue (`self.Make Viewer (With Transform)` (`KismetMathLibrary.MakeTransform` (`Actor.K2_GetActorLocation` (`self.GetOwner`)) Direction)))
  (`SpacialViewer.ShowForward` _returnvalue `View Mode`))

(fn `Show Forward (With Transform)`
  (params (`View Mode` :type "EDirectionViewMode Enum" :default "Vector") (Transform :type "Transform Structure"))
  (bind _returnvalue (`self.Make Viewer (With Transform)` Transform))
  (`SpacialViewer.ShowForward` _returnvalue `View Mode`))

(fn `Show Orientation`
  (params (_useGnomon :type Boolean))
  (`SpacialViewer.ShowOrientation` (`self.Parent_View`) _useGnomon))

(fn `Show Orientation (At Direction)`
  (params (Rotation :type "Rotator Structure") (_useGnomon :type Boolean))
  (bind _returnvalue (`self.Make Viewer (With Transform)` (`KismetMathLibrary.MakeTransform` (`Actor.K2_GetActorLocation` (`self.GetOwner`)) Rotation)))
  (`SpacialViewer.ShowOrientation` _returnvalue _useGnomon))

(fn `Show Orientation (With Transform)`
  (params (Transform :type "Transform Structure") (_useGnomon :type Boolean))
  (bind _returnvalue (`self.Make Viewer (With Transform)` Transform))
  (`SpacialViewer.ShowOrientation` _returnvalue _useGnomon))

(fn `Show Position`
  (`SpacialViewer.ShowPosition` (`self.Parent_View`)))

(fn `Show Position (At Location)`
  (params (Location :type "Vector Structure"))
  (bind _returnvalue (`self.Make Viewer (With Transform)` (`KismetMathLibrary.MakeTransform` Location)))
  (`SpacialViewer.ShowPosition` _returnvalue))

(fn `Show Right`
  (params (`View Mode` :type "EDirectionViewMode Enum" :default "Vector"))
  (`SpacialViewer.ShowRight` (`self.Parent_View`) `View Mode`))

(fn `Show Right (At Direction)`
  (params (Direction :type "Rotator Structure (by ref)") (`View Mode` :type "EDirectionViewMode Enum" :default "Vector"))
  (bind _returnvalue (`self.Make Viewer (With Transform)` (`KismetMathLibrary.MakeTransform` (`Actor.K2_GetActorLocation` (`self.GetOwner`)) Direction)))
  (`SpacialViewer.ShowRight` _returnvalue `View Mode`))

(fn `Show Right (With Transform)`
  (params (Transform :type "Transform Structure") (`View Mode` :type "EDirectionViewMode Enum" :default "Vector"))
  (bind _returnvalue (`self.Make Viewer (With Transform)` Transform))
  (`SpacialViewer.ShowRight` _returnvalue `View Mode`))

(fn `Show Scale`
  (`SpacialViewer.ShowScale` (`self.Parent_View`)))

(fn `Show Scale (With Transform)`
  (params (Transform :type "Transform Structure"))
  (bind _returnvalue (`self.Make Viewer (With Transform)` Transform))
  (`SpacialViewer.ShowScale` _returnvalue))

(fn `Show Transform`
  (params (_useGnomon :type Boolean) (`With Scale` :type Boolean))
  (`SpacialViewer.ShowTransform` (`self.Parent_View`) _useGnomon `With Scale`))

(fn `Show Transform (With Transform)`
  (params (Transform :type "Transform Structure") (_useGnomon :type Boolean) (`With Scale` :type Boolean))
  (bind _returnvalue (`self.Make Viewer (With Transform)` Transform))
  (`SpacialViewer.ShowTransform` _returnvalue _useGnomon `With Scale`))

(fn `Show Up`
  (params (`View Mode` :type "EDirectionViewMode Enum" :default "Vector"))
  (`SpacialViewer.ShowUp` (`self.Parent_View`) `View Mode`))

(fn `Show Up (At Direction)`
  (params (Direction :type "Rotator Structure") (`View Mode` :type "EDirectionViewMode Enum" :default "Vector"))
  (bind _returnvalue (`self.Make Viewer (With Transform)` (`KismetMathLibrary.MakeTransform` (`Actor.K2_GetActorLocation` (`self.GetOwner`)) Direction)))
  (`SpacialViewer.ShowUp` _returnvalue `View Mode`))

(fn `Show Up (With Transform)`
  (params (Transform :type "Transform Structure") (`View Mode` :type "EDirectionViewMode Enum" :default "Vector"))
  (bind _returnvalue (`self.Make Viewer (With Transform)` Transform))
  (`SpacialViewer.ShowUp` _returnvalue `View Mode`))