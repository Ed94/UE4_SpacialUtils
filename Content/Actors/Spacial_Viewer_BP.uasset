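; Spacial_Viewer_BP is a visual helper actor that displays chosen parts of a transform: position, direction axes, orientation and scale.
; ShowView switches on a view option and calls the matching Show function, which turns on the relevant components.
; A view mode selects axis vectors, planes or both for directions.
; The functions only reveal components, except ShowTransform, which sets the scale cube's visibility from WithScale.
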(fn `Show Forward`
  (params (`View Mode` :type "/Game/Components/Assets/EDirectionView_Mode Enum" :default "NewEnumerator0"))
  (switch `/Game/Components/Assets/EDirectionView_Mode` `View Mode`
    (:`NewEnumerator0`
      (`SceneComponent.SetVisibility` (`self.Forward`) true true))
    (:`NewEnumerator1`
      (`SceneComponent.SetVisibility` (`self.Front`) true true))
    (:`NewEnumerator2`
      (`SceneComponent.SetVisibility` (`self.Forward`) true true)
      (`SceneComponent.SetVisibility` (`self.Front`) true true))))

(fn `Show Orientation`
  (params (`View Mode` :type "/Game/Components/Assets/EDirectionView_Mode Enum" :default "NewEnumerator0"))
  (bind _forward (`self.Forward`))
  (switch `/Game/Components/Assets/EDirectionView_Mode` `View Mode`
    (:`NewEnumerator0`
      (`SceneComponent.SetVisibility` _forward true true)
      (`SceneComponent.SetVisibility` (`self.Right`) true true)
      (`SceneComponent.SetVisibility` (`self.Up`) true true))
    (:`NewEnumerator1`
      (`SceneComponent.SetVisibility` (`self.Floor`) true true)
      (`SceneComponent.SetVisibility` (`self.Face`) true true)
      (`SceneComponent.SetVisibility` (`self.Side`) true true))
    (:`NewEnumerator2`
      (`SceneComponent.SetVisibility` _forward true true)
      (`SceneComponent.SetVisibility` (`self.Right`) true true)
      (`SceneComponent.SetVisibility` (`self.Side`) true true)
      (`SceneComponent.SetVisibility` (`self.Up`) true true)
      (`SceneComponent.SetVisibility` (`self.Floor`) true true)
      (`SceneComponent.SetVisibility` (`self.Face`) true true))))

(fn `Show Position`
  (`SceneComponent.SetVisibility` (`self.Position`) true true))

(fn `Show Right`
  (params (`View Mode` :type "/Game/Components/Assets/EDirectionView_Mode Enum" :default "NewEnumerator0"))
  (switch `/Game/Components/Assets/EDirectionView_Mode` `View Mode`
    (:`NewEnumerator0`
      (`SceneComponent.SetVisibility` (`self.Right`) true true))
    (:`NewEnumerator1`
      (`SceneComponent.SetVisibility` (`self.Side`) true true))
    (:`NewEnumerator2`
      (`SceneComponent.SetVisibility` (`self.Right`) true true)
      (`SceneComponent.SetVisibility` (`self.Side`) true true))))

(fn `Show Scale`
  (`SceneComponent.SetVisibility` (`self.Scale Cube`) true true))

(fn `Show Transform`
  (params (`With Scale` :type Boolean) (`Orientation VIew` :type "/Game/Components/Assets/EDirectionView_Mode Enum" :default "NewEnumerator0"))
  (bind _face (`self.Face`))
  (switch `/Game/Components/Assets/EDirectionView_Mode` `Orientation VIew`
    (:`NewEnumerator0`
      (`SceneComponent.SetVisibility` (`self.Right`) true false)
      (`SceneComponent.SetVisibility` (`self.Up`) true false)
      (`SceneComponent.SetVisibility` (`self.Forward`) true false)
      (`SceneComponent.SetVisibility` (`self.Location Sphere`) true false))
    (:`NewEnumerator1`
      (`SceneComponent.SetVisibility` _face true false)
      (`SceneComponent.SetVisibility` (`self.Side`) true false)
      (`SceneComponent.SetVisibility` (`self.Floor`) true false)
      (`SceneComponent.SetVisibility` (`self.Location Sphere`) true false))
    (:`NewEnumerator2`
      (`SceneComponent.SetVisibility` _face true false)
      (`SceneComponent.SetVisibility` (`self.Location Sphere`) true false)
      (`SceneComponent.SetVisibility` (`self.Right`) true false)
      (`SceneComponent.SetVisibility` (`self.Side`) true false)
      (`SceneComponent.SetVisibility` (`self.Up`) true false)
      (`SceneComponent.SetVisibility` (`self.Floor`) true false)
      (`SceneComponent.SetVisibility` (`self.Forward`) true false)))
  (`SceneComponent.SetVisibility` (`self.Scale Cube`) `With Scale` false))

(fn `Show Up`
  (params (`View Mode` :type "/Game/Components/Assets/EDirectionView_Mode Enum" :default "NewEnumerator0"))
  (bind _floor (`self.Floor`))
  (switch `/Game/Components/Assets/EDirectionView_Mode` `View Mode`
    (:`NewEnumerator0`
      (`SceneComponent.SetVisibility` (`self.Up`) true true))
    (:`NewEnumerator1`
      (`SceneComponent.SetVisibility` _floor true true))
    (:`NewEnumerator2`
      (`SceneComponent.SetVisibility` _floor true true)
      (`SceneComponent.SetVisibility` (`self.Up`) true true))))

(fn `Show View`
  (params (`View Option` :type "/Game/Components/Assets/ESViewer_ViewOption Enum" :default "NewEnumerator3") (`Direction View Mode` :type "/Game/Components/Assets/EDirectionView_Mode Enum" :default "NewEnumerator0") (`With Scale` :type Boolean))
  (switch `/Game/Components/Assets/ESViewer_ViewOption` `View Option`
    (:`NewEnumerator3`
      (`self.Show Position`))
    (:`NewEnumerator0`
      (`self.Show Forward` `Direction View Mode`))
    (:`NewEnumerator2`
      (`self.Show Right` `Direction View Mode`))
    (:`NewEnumerator1`
      (`self.Show Up` `Direction View Mode`))
    (:`NewEnumerator4`
      (`self.Show Orientation` `Direction View Mode`))
    (:`NewEnumerator5`
      (`self.Show Scale`))
    (:`NewEnumerator6`
      (`self.Show Transform` `With Scale` `Direction View Mode`))))

(fn `UserConstructionScript`)